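; BP_PlatformTrigger is a trigger actor for an endless runner that spawns new platform tiles and removes old ones.
; It caches GM_EndlessRunner on BeginPlay.
; Any overlap with its Box tells that game mode to spawn a tile at the newest platform's SpawnPoint.
; If the overlapping actor is tagged Platform, it is destroyed after a short delay.
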(event `self.ReceiveBeginPlay`
  (bind _asgm_endless_runner (cast `/Game/GM_EndlessRunner` (`GameplayStatics.GetGameMode`)))
  (set `self.GameModeRef` _asgm_endless_runner))

(event `self.Box.OnComponentBeginOverlap`
  (params (OverlappedComponent :type "PrimitiveComponent Object Reference") (OtherActor :type "Actor Object Reference") (OtherComp :type "PrimitiveComponent Object Reference") (OtherBodyIndex :type Integer) (bFromSweep :type Boolean) (SweepResult :type "HitResult Structure (by ref)"))
  (bind _gamemoderef (`self.GameModeRef`))
  (`/Game/GM_EndlessRunner.Spawn Tile` _gamemoderef (`SceneComponent.K2_GetComponentLocation` (`/Game/BP_Platform.Spawn Point` (`/Game/GM_EndlessRunner.NewPlatform` _gamemoderef))))
  (if (`self.ActorHasTag` OtherActor "Platform")
    (`KismetSystemLibrary.Delay` 1.0)
    (`self.K2_DestroyActor` OtherActor)))

(fn `UserConstructionScript`)
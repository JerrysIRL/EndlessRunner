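; Endless runner game mode, by its name, that builds and tracks the chain of BP_Platform tiles making up the track.
; On BeginPlay it spawns a tile at the world origin, then chains more, each at the previous tile's SpawnPoint.
; MovePlatform supports reusing tiles by relocating a given platform, storing it as the newest and returning its SpawnPoint location.
; Nothing in this graph calls MovePlatform.
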(event `self.ReceiveBeginPlay`
  (`self.Spawn Tile` (0.0 0.0 0.0))
  (for _ (range 15)
    (`self.Spawn Tile` (`SceneComponent.K2_GetComponentLocation` (`/Game/BP_Platform.Spawn Point` (`self.NewPlatform`))))))

(fn `Move Platform`
  (params (Platform :type "Actor Object Reference") (Position :type "Vector Structure"))
  (returns (`Next Position` :type "Vector Structure"))
  (`self.K2_SetActorLocation` Platform Position false false)
  (bind _asbp_platform (cast `/Game/BP_Platform` Platform))
  (bind _output_get (set `self.NewPlatform` _asbp_platform))
  (return (`SceneComponent.K2_GetComponentLocation` (`/Game/BP_Platform.Spawn Point` _output_get))))

(fn `Spawn Tile`
  (params (Position :type "Vector Structure"))
  (returns (Platform :type "/Game/BP_Platform Object Reference"))
  (bind _returnvalue (`|SpawnActorFromClass` "/Game/BP_Platform.BP_Platform_C" (`KismetMathLibrary.MakeTransform` Position) "Undefined" "OverrideRootScale" null null))
  (bind _output_get (set `self.NewPlatform` _returnvalue))
  (return _output_get))

(fn `UserConstructionScript`)
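; Input receiver for a local two-player endless runner, routing one set of inputs to both player pawns.
; On BeginPlay it takes the first two BP_ExtendedPawn actors as Player One and Two, then creates WB_GameUI with both pawns and GM_EndlessRunner, removing it when destroyed.
; Separate keys, axes and actions forward jump, movement and crouch to each pawn, with crouch release resetting rotation.
; F1 runs the FPS stat console command.
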(event `self.ReceiveBeginPlay`
  (bind _outactors (`GameplayStatics.GetAllActorsOfClass` "/Game/BluePrints/BP_ExtendedPawn.BP_ExtendedPawn_C"))
  (set `self.PlayerOne` (`|GetArrayItem` _outactors))
  (set `self.PlayerTwo` (`|GetArrayItem` _outactors 1))
  ;[1 1 1] Player UI
  (bind _returnvalue (`|CreateWidget` "/Game/BluePrints/WB_GameUI.WB_GameUI_C"))
  (set `/Game/BluePrints/WB_GameUI.P2Ref` (`self.PlayerTwo`) _returnvalue)
  (set `/Game/BluePrints/WB_GameUI.P1Ref` (`self.PlayerOne`) _returnvalue)
  (bind _asgm_endless_runner (cast `/Game/GM_EndlessRunner` (`GameplayStatics.GetGameMode`)))
  (set `/Game/BluePrints/WB_GameUI.GameMode` _asgm_endless_runner _returnvalue)
  (`UserWidget.AddToPlayerScreen` _returnvalue 0))

(event `self.ReceiveDestroyed`
  ;[1 1 1] Player UI
  (`Widget.RemoveFromParent` (stale `self.ReceiveBeginPlay` _returnvalue)))

(event `Key|W`
  (params (Key :type "Key Structure"))
  (bind _playerone (`self.PlayerOne`))
  ;[1 1 1] Player1
  (:`Pressed`
    (`/Engine/EditorBlueprintResources/StandardMacros.IsValid` _playerone
      (:`Is Valid`
        (`Character.Jump` _playerone)))))

(event `Key|Up`
  (params (Key :type "Key Structure"))
  (bind _playertwo (`self.PlayerTwo`))
  ;[1 1 1] Player2
  (:`Pressed`
    (`/Engine/EditorBlueprintResources/StandardMacros.IsValid` _playertwo
      (:`Is Valid`
        (`Character.Jump` _playertwo)))))

(event `InputAxis|Move Right / Left`
  (params (AxisValue :type "Float (single-precision)"))
  (bind _playerone (`self.PlayerOne`))
  ;[1 1 1] Player1
  (`/Engine/EditorBlueprintResources/StandardMacros.IsValid` _playerone
    (:`Is Valid`
      (`ExtendedPawn.Move` _playerone AxisValue))))

(event `InputAxis|Move Right/LeftP2`
  (params (AxisValue :type "Float (single-precision)"))
  (bind _playertwo (`self.PlayerTwo`))
  ;[1 1 1] Player2
  (`/Engine/EditorBlueprintResources/StandardMacros.IsValid` _playertwo
    (:`Is Valid`
      (`ExtendedPawn.Move` _playertwo AxisValue))))

(event `InputAction|CrouchP2`
  (params (Key :type "Key Structure"))
  (bind _playertwo (`self.PlayerTwo`))
  ;[1 1 1] Player2
  (:`Pressed`
    (`/Engine/EditorBlueprintResources/StandardMacros.IsValid` _playertwo
      (:`Is Valid`
        (`ExtendedPawn.CharCrouch` _playertwo))))
  (:`Released`
    (`ExtendedPawn.ResetRot` _playertwo)))

(event `InputAction|Crouch`
  (params (Key :type "Key Structure"))
  (bind _playerone (`self.PlayerOne`))
  ;[1 1 1] Player1
  (:`Pressed`
    (`/Engine/EditorBlueprintResources/StandardMacros.IsValid` _playerone
      (:`Is Valid`
        (`ExtendedPawn.CharCrouch` _playerone))))
  (:`Released`
    (`ExtendedPawn.ResetRot` _playerone)))

(event `Key|F1`
  (params (Key :type "Key Structure"))
  (:`Pressed`
    (`KismetSystemLibrary.ExecuteConsoleCommand` "stat fps" null)))

(fn `UserConstructionScript`)